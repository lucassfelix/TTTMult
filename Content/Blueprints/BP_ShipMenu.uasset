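; BP_ShipMenu is a ship actor, apparently for the menu, that gently rocks its Body in place.
; BeginPlay sets the Body's starting rotation, and Tick adds a small sine-driven local roll each frame.
; ShipSpeed serves as a frame counter, multiplied by DeltaSeconds to form the sine phase.
; Disconnected nodes that would move the ship and destroy it beyond an X limit never run.
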(event EventBeginPlay
  (Transformation|SetRelativeRotation (Variables|Default|GetBody) "0.000000,-90.000000,-2.500000" false false))

(event EventTick
  (params (DeltaSeconds :type Float%20%28single-precision%29))
  (bind _result (Math|Float|IncrementFloat (Variables|Default|GetShipSpeed))
    (:%20%20
      (Transformation|AddLocalRotation (Variables|Default|GetBody) (Math|Rotator|MakeRotator (* (Math|Trig|Sin(Radians) (* (* _result DeltaSeconds) 1.0)) 0.05) 0.0 0.0) false false))))

(fn ConstructionScript)