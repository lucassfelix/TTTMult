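; BP_Ship is a ship actor that accelerates along a straight path and destroys itself once out of bounds.
; BeginPlay sets the Body's starting orientation, then each Tick increments ShipSpeed and applies it as an unswept local Y offset, independent of frame time.
; The same counter, scaled by delta time, drives a sine-based roll wobble.
; The actor is destroyed when the Body's absolute world X passes a fixed limit.
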(event EventBeginPlay
  (Transformation|SetRelativeRotation (Variables|Default|GetBody) "0.000000,-90.000000,-2.500000" false false))

(event EventTick
  (params (DeltaSeconds :type Float%20%28single-precision%29))
  (bind _result (Math|Float|IncrementFloat (Variables|Default|GetShipSpeed))
    (:%20%20
      (Transformation|AddLocalRotation (Variables|Default|GetBody) (Math|Rotator|MakeRotator (* (Math|Trig|Sin(Radians) (* (* _result DeltaSeconds) 1.0)) 0.05) 0.0 0.0) false false)
      (bind _output_get (Variables|Default|SetLocationOffset (Math|Vector|MakeVector 0.0 (Variables|Default|GetShipSpeed) 0.0)))
      (Transformation|AddLocalOffset (Variables|Default|GetBody) _output_get false false)
      (if (> (Math|Float|Absolute(Float) (.x (Transformation|GetWorldLocation (Variables|Default|GetBody)))) 9.8e+02)
        (Actor|DestroyActor)))))

(fn ConstructionScript)