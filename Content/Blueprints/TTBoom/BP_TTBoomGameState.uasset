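; Game state for TTBoom, a tic-tac-toe game where ball hits claim board pieces for team X or O.
; On BeginPlay it gathers and sorts all board pieces and caches the first player controller's HUD.
; A hit on an empty piece sets its mark and material, then runs an endgame check.
; A finished game triggers a multicast that prints the result and notifies the HUD only when X wins.
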(event Custom|Multicast_GameEnded
  (params (WhoWon :type EPieceType%20Enum :default "P_X"))
  (switch Utilities|FlowControl|Switch|SwitchonEPieceType WhoWon
    (:P_X
      (Development|PrintString "X ganhou!")
      (Default|PlayerWon (Variables|Default|GetGameHUD)))
    (:P_O
      (Development|PrintString "O ganhou!"))
    (:P_Empty
      (Development|PrintString "Empate.!"))))

(event Custom|OnReceiveBallHit
  (params (Hit :type Board%20Piece%20Object%20Reference) (Team :type EPlayerTeam%20Enum :default "P_X"))
  (bind _returnvalue (Utilities|Select :Index Team :P_X "P_X" :P_O "P_O" :P_Empty "P_Empty"))
  (if (Utilities|Enum|Equal(Enum) (Class|BoardPiece|GetCurrentPiece Hit) "P_Empty")
    (Class|BoardPiece|SetCurrentPiece Hit _returnvalue)
    (Class|BoardPiece|OnChangeMaterial Hit _returnvalue)
    (bind _returnvalue_2 (Class|TTBoomGameState|CheckEndgame))
    (if (not (== _returnvalue_2 -1))
      (CallFunction|MulticastGameEnded (Utilities|Select :Index _returnvalue_2 :Option%200 "P_Empty" :Option%201 "P_X" :Option%202 "P_O")))))

(event EventBeginPlay
  (bind _outactors (Actor|GetAllActorsOfClass "/Game/Blueprints/BP_BoardPiece.BP_BoardPiece_C"))
  (Variables|Default|SetBoardPieces _outactors)
  (Class|TTBoomGameState|SortPieces)
  (bind _asbp_cannon_player_controller (Utilities|Casting|CastToBP_CannonPlayerController (Game|GetPlayerController 0)))
  (Variables|Default|SetGameHUD (Variables|/Game/Blueprints/TTBoom/BP_CannonPlayerController.BP_CannonPlayerController_C|GetGameHUD _asbp_cannon_player_controller)))

(fn ConstructionScript)