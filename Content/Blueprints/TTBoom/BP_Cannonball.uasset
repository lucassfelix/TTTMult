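; Cannonball projectile actor for TTBoom that reports which team's shot struck a board piece.
; On a server-side hit, it prints the struck actor and the ShotBy team (X, O or Empty).
; It then passes ShotBy and the struck BoardPiece to the CannonPlayerController at player index 0 and destroys itself.
; If either cast fails, the ball is left in place.
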(event Collision|EventHit
  (params (MyComp :type Primitive%20Component%20Object%20Reference) (Other :type Actor%20Object%20Reference) (OtherComp :type Primitive%20Component%20Object%20Reference) (bSelfMoved :type Boolean) (HitLocation :type Vector :default "0, 0, 0") (HitNormal :type Vector :default "0, 0, 0") (NormalImpulse :type Vector :default "0, 0, 0") (Hit :type Hit%20Result%20Structure%20%28by%20ref%29))
  (bind _shotby (Variables|Default|GetShotBy))
  (if (Networking|IsServer)
    (Development|PrintString (Utilities|String|ToString(Text) (Utilities|Text|FormatText "Hit: {Name} 
I was shot by: {Shot}" Other (Utilities|Select :Index _shotby :P_X (Utilities|Text|ToText(String) "X") :P_O "O" :P_Empty "Empty"))))
    (bind _ascannon_player_controller (Utilities|Casting|CastToCannonPlayerController (Game|GetPlayerController 0)))
    (bind _asboard_piece (Utilities|Casting|CastToBoardPiece Other))
    (Class|CannonPlayerController|ReceiveonBallHit _ascannon_player_controller _shotby _asboard_piece)
    (Actor|DestroyActor)))

(fn ConstructionScript)