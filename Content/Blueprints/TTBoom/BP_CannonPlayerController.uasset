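; Player controller for TTBoom's X-versus-O cannon game, creating the HUD and relaying shots and board hits to the server.
; Shoot input resets the height step when the turn or free-mode cooldown permits.
; The server rechecks that rule with slight cooldown leniency, spawns and launches the team-tagged cannonball, multicasts its sound, resets shot timers and flips the turn.
; Board-piece hits go through a server event to the game state.
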(event Custom|Server_SpawnCannonball
  (params (StartLocation :type Transform) (LaunchVelocity :type Vector) (Team :type EPlayerTeam%20Enum :default "P_X"))
  (bind _returnvalue (Class|TTBoomGameState|GetTTBoomGameState))
  (bind _returnvalue_2 (Class|TTBoomGameState|GetTTBoomGameState))
  (bind (_location _rotation) (Math|Transform|BreakTransform StartLocation))
  (switch Utilities|FlowControl|Switch|SwitchonEPlayMode (Class|TTBoomGameState|GetPlayMode _returnvalue_2)
    (:TurnBased
      (bind _asttboom_player_state (Utilities|Casting|CastToTTBoomPlayerState (Variables|Default|GetPlayerState)))
      (if (Utilities|Enum|Equal(Enum) (Class|TTBoomGameState|GetCurrentPlayer _returnvalue_2) (Variables|/Script/TTTMult.TTBoomPlayerState|GetPlayerTeam _asttboom_player_state))
        (bind _returnvalue_3 (Game|SpawnActorfromClass "/Game/Blueprints/TTBoom/BP_Cannonball.BP_Cannonball_C" (Math|Transform|MakeTransform _location _rotation "0.400000,0.400000,0.400000") "Undefined" 0 0 :!label _label))
        (Development|PrintString (Utilities|String|ToString(Boolean) (Networking|IsServer)))
        (CallFunction|MulticastCannonballSound)
        (Variables|/Script/TTTMult.Cannonball|SetShotBy _returnvalue_3 Team)
        (Physics|SetPhysicsLinearVelocity (Variables|/Game/Blueprints/TTBoom/BP_Cannonball.BP_Cannonball_C|GetCannonballMesh _returnvalue_3) LaunchVelocity false "None")
        (Variables|Default|SetTimeBetweenLastShot_Server 0.0)
        (Variables|Default|SetTimeBetweenLastShot_Client 0.0)
        (Class|TTBoomGameState|SetCurrentPlayerTurn _returnvalue (Utilities|Select :Index (Variables|/Script/TTTMult.TTBoomGameState|GetCurrentPlayerTurn _returnvalue) :P_X "P_O" :P_O "P_X" :P_Empty "P_Empty"))))
    (:FreeMode
      (if (> (Variables|Default|GetTimeBetweenLastShot_Server) (- (Variables|Default|GetCooldown) 0.2))
        (goto _label)))))

(event Custom|Server_OnBallHit
  (params (HitPiece :type Board%20Piece%20Object%20Reference) (BallTeam :type EPlayerTeam%20Enum :default "P_X"))
  (Development|PrintString "Called Server on Ball Hit" true true "(R=1.000000,G=0.108869,B=0.000000,A=1.000000)")
  (bind _asbp_ttboom_game_state (Utilities|Casting|CastToBP_TTBoomGameState (Game|GetGameState)))
  (Default|OnReceiveBallHit _asbp_ttboom_game_state HitPiece BallTeam))

(event Custom|Multicast_CannonballSound
  (AddComponent|AddAudioComponent false)
  (Development|PrintString "Atirei!"))

(event Input|EnhancedActionEvents|EnhancedInputActionIA_ShootAction
  (params (ActionValue :type Boolean) (ElapsedSeconds :type Float%20%28double-precision%29) (TriggeredSeconds :type Float%20%28double-precision%29) (InputAction :type Input%20Action%20Object%20Reference :default "/Game/Input/TTBoom/Actions/IA_ShootAction.IA_ShootAction"))
  (bind _returnvalue (Class|TTBoomGameState|GetTTBoomGameState))
  (:Started
    (switch Utilities|FlowControl|Switch|SwitchonEPlayMode (Class|TTBoomGameState|GetPlayMode _returnvalue)
      (:TurnBased
        (bind _asttboom_player_state (Utilities|Casting|CastToTTBoomPlayerState (Variables|Default|GetPlayerState)))
        (if (Utilities|Enum|Equal(Enum) (Variables|/Script/TTTMult.TTBoomPlayerState|GetPlayerTeam _asttboom_player_state) (Class|TTBoomGameState|GetCurrentPlayer _returnvalue))
          (Variables|Default|SetHeightCurrentStep (Variables|Default|GetHeightInitialStep))))
      (:FreeMode
        (if (> (Variables|Default|GetTimeBetweenLastShot_Client) (Variables|Default|GetCooldown))
          (Variables|Default|SetHeightCurrentStep (Variables|Default|GetHeightInitialStep)))))))

(event EventOnSpawnCannonball
  (params (LaunchVelocity :type Vector :default "0, 0, 0") (Team :type EPlayerTeam%20Enum :default "P_X") (StartLocation :type Transform))
  (CallFunction|ServerSpawnCannonball StartLocation LaunchVelocity Team))

(event EventBeginPlay
  (bind _returnvalue (Game|GetPlayerController 0))
  (bind _returnvalue_2 (UserInterface|CreateWidget "/Game/UI/WBP_HUD.WBP_HUD_C" _returnvalue))
  (bind _output_get (Variables|Default|SetGameHUD _returnvalue_2))
  (UserInterface|Viewport|AddtoViewport _output_get 0)
  (Input|SetInputModeGameOnly _returnvalue false)
  (Variables|Default|SetbShowMouseCursor false))

(event EventOnBallHit
  (params (ShotBy :type EPlayerTeam%20Enum :default "P_X") (Other :type Actor%20Object%20Reference))
  (bind _asboard_piece (Utilities|Casting|CastToBoardPiece Other))
  (CallFunction|ServeronBallHit _asboard_piece ShotBy))

(fn ConstructionScript)

(fn OnRepTimeBetweenShot)