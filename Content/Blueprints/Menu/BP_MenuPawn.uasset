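; BP_MenuPawn is a menu pawn that animates its camera between menu views.
; On BeginPlay it caches the camera's relative location and rotation as the home transform.
; JoinButtonClicked slides the camera along Y to a fixed offset, keeping its height and rotation, and BackButtonClicked returns it to the cached transform.
; Both moves use MoveComponentTo with timed ease-in and ease-out.
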(event Custom|JoinButtonClicked
  (bind _camera (Variables|Default|GetCamera))
  (Components|MoveComponentTo _camera (Math|Vector|MakeVector 0.0 1.5e+03 (.z (Variables|/Script/Engine.SceneComponent|GetRelativeLocation _camera))) (Variables|/Script/Engine.SceneComponent|GetRelativeRotation _camera) true true 1.5 false))

(event Custom|BackButtonClicked
  (Components|MoveComponentTo (Variables|Default|GetCamera) (Variables|Default|GetOriginalLocation) (Variables|Default|GetOriginalRotation) true true 1.5 false))

(event EventBeginPlay
  (bind _camera (Variables|Default|GetCamera))
  (bind _output_get (Variables|Default|SetOriginalLocation (Variables|/Script/Engine.SceneComponent|GetRelativeLocation _camera)))
  (bind _output_get_2 (Variables|Default|SetOriginalRotation (Variables|/Script/Engine.SceneComponent|GetRelativeRotation _camera)))
  (Transformation|SetRelativeLocationAndRotation _camera _output_get _output_get_2 false false))

(fn ConstructionScript)